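; Boss actor Blueprint that drives a health bar widget and shows the game clear screen.
; Every tick it casts its Health component's widget to the health widget and sets the bar percent from current over max HP.
; OnGameClear enables the mouse cursor and mouse-over events, then creates the WBP_GameClear widget and adds it to the viewport.
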(event `self.OnGameClear`
  (bind _returnvalue (`GameplayStatics.GetPlayerController` 0))
  (bind _output_get (set `PlayerController.bShowMouseCursor` true _returnvalue))
  (set `PlayerController.bEnableMouseOverEvents` _output_get _returnvalue)
  (bind _returnvalue_2 (`|CreateWidget` "/Game/LMBCPP/UI/WBP_GameClear.WBP_GameClear_C"))
  (`UserWidget.AddToViewport` _returnvalue_2 0))

(event `self.ReceiveTick`
  (params (DeltaSeconds :type "Float (single-precision)"))
  (bind _ashealth (cast `/Game/LMBCPP/UI/health` (`WidgetComponent.GetWidget` (`self.Health`))))
  (`ProgressBar.SetPercent` (`/Game/LMBCPP/UI/health.healthbar` _ashealth) (/ (`self.CurrentHp`) (`self.MaxHp`))))

(fn `UserConstructionScript`)